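; Blacksmith is an NPC Blueprint that starts a dialogue when it is interacted with.
; Both the construction script and BeginPlay cast its AI controller to NPC_AI and pass it the character's XdiaDialogueTree.
; The Xdiainteractfunc event then calls StartDialogue on that controller, which, per the graph's note, runs the behavior tree.
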(event EventBeginPlay
  ;[1 1 1] Adds "NPC_AI" AI controller as a property to the NPC's blueprint, also sets dialogue tree to the AI controller
  (bind _asnpc_ai (Utilities|Casting|CastToNPC_AI (AI|GetAIController self)))
  (Variables|/Game/Playercore/Blueprints/xdialogue/NPC_AI.NPC_AI_C|SetXdiaDialogueTree _asnpc_ai (Variables|Default|GetXdiaDialogueTree)))

(event EventXdiainteractfunc
  ;[1 1 1] When an interact is called on the character, it will execute Start Dialogue event, which will run the behavior tree
  (bind _asnpc_ai (Utilities|Casting|CastToNPC_AI (AI|GetAIController self)))
  (Default|StartDialogue _asnpc_ai))

(fn ConstructionScript
  ;[1 1 1] Adds "NPC_AI" AI controller as a property to the NPC's blueprint, also sets dialogue tree to the AI controller
  (bind _asnpc_ai (Utilities|Casting|CastToNPC_AI (AI|GetAIController self)))
  (Variables|/Game/Playercore/Blueprints/xdialogue/NPC_AI.NPC_AI_C|SetXdiaDialogueTree _asnpc_ai (Variables|Default|GetXdiaDialogueTree)))